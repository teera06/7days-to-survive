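; Main networked player character blueprint, handling player setup, weapon selection and aiming.
; BeginPlay applies mesh, name and spawn location from BP_STSInstance through Server/Mult events, repeated once on first move input, and adds local minimap and blood-FX UI.
; Number keys select quick slots, or directly swap weapons in CharDevelopMode.
; Zoom switches view target to the weapon and shows the crosshair; Tick undoes this while hit or dead.
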(event `MultName`
  ;[1 1 1] 이름 동기화
  (`TextRenderComponent.K2_SetText` (`self.NameText`) (`self.PlayerName`)))

(event `MultMesh`
  ;[1 1 1] 메시 동기화
  (bind _asbp_stsinstance (cast `/Game/STS/BP_STSInstance` (`GameplayStatics.GetGameInstance`)))
  (bind _returnvalue (`C_STSInstance.GetPlayerSpawnMesh` _asbp_stsinstance))
  (`SkeletalMeshComponent.SetSkeletalMeshAsset` (`self.Mesh`) (`|GetArrayItem` _returnvalue (`KismetMathLibrary.Conv_ByteToInt` (`self.characterResultMesh`)))))

(event `EnhancedInput|/Game/Level/TestLevel/CharTest/Player/Input/Action/IA_NoWeapon`
  (params (ActionValue :type Boolean) (ElapsedSeconds :type "Float (double-precision)") (TriggeredSeconds :type "Float (double-precision)") (InputAction :type "InputAction Object Reference" :default "/Game/Level/TestLevel/CharTest/Player/Input/Action/IA_NoWeapon.IA_NoWeapon"))
  (:`Started`
    ;[1 1 1] 무기 변경
    (if (and (`self.IsHitCpp`) (`self.IsPlayerDieCpp`))
      _
      (elif (`self.CharDevelopMode`)
        (`self.ChangeNoWeaponServer`)))))

(event `EnhancedInput|/Game/Level/TestLevel/CharTest/Player/Input/Action/IA_number3Weapon`
  (params (ActionValue :type Boolean) (ElapsedSeconds :type "Float (double-precision)") (TriggeredSeconds :type "Float (double-precision)") (InputAction :type "InputAction Object Reference" :default "/Game/Level/TestLevel/CharTest/Player/Input/Action/IA_number3Weapon.IA_number3Weapon"))
  ;[1 1 1] 무기 변경
  (:`Started`
    (if (and (`self.IsHitCpp`) (`self.IsPlayerDieCpp`))
      _
      (elif (`self.CharDevelopMode`)
        (`self.ChangeSlotMeshServer` "RAxe" "/Game/Level/TestLevel/CharTest/Axe_OneHanded/Axe_StaticMesh.Axe_StaticMesh")
        (else
          (`self.OnQuickSlotSelected` 2))))))

(event `EnhancedInput|/Game/Level/TestLevel/CharTest/Player/Input/Action/IA_number6Weapon`
  (params (ActionValue :type Boolean) (ElapsedSeconds :type "Float (double-precision)") (TriggeredSeconds :type "Float (double-precision)") (InputAction :type "InputAction Object Reference" :default "/Game/Level/TestLevel/CharTest/Player/Input/Action/IA_number6Weapon.IA_number6Weapon"))
  ;[1 1 1] 무기 변경
  (:`Started`
    (if (and (`self.IsHitCpp`) (`self.IsPlayerDieCpp`))
      _
      (elif (`self.CharDevelopMode`)
        (`self.ChangeSlotSkeletalServer` "RRifle2")
        (else
          (`self.OnQuickSlotSelected` 5))))))

(event `ServerName`
  ;[1 1 1] 이름 동기화
  (`self.MultName`))

(event `Server`
  ;[1 1 1] 메시 동기화
  (`self.MultMesh`))

(event `EnhancedInput|/Game/Level/TestLevel/CharTest/Player/Input/Action/IA_number1Weapon`
  (params (ActionValue :type Boolean) (ElapsedSeconds :type "Float (double-precision)") (TriggeredSeconds :type "Float (double-precision)") (InputAction :type "InputAction Object Reference" :default "/Game/Level/TestLevel/CharTest/Player/Input/Action/IA_number1Weapon.IA_number1Weapon"))
  (:`Started`
    ;[1 1 1] 무기 변경
    (if (and (`self.IsHitCpp`) (`self.IsPlayerDieCpp`))
      _
      (elif (`self.CharDevelopMode`)
        (`self.ChangeSlotMeshServer` "RBat" "/Game/Level/TestLevel/CharTest/Bat/bat1.bat1")
        (else
          (`self.OnQuickSlotSelected` 0))))))

(event `EnhancedInput|/Game/Level/TestLevel/CharTest/Player/Input/Action/IA_numver4Weapon`
  (params (ActionValue :type Boolean) (ElapsedSeconds :type "Float (double-precision)") (TriggeredSeconds :type "Float (double-precision)") (InputAction :type "InputAction Object Reference" :default "/Game/Level/TestLevel/CharTest/Player/Input/Action/IA_numver4Weapon.IA_numver4Weapon"))
  ;[1 1 1] 무기 변경
  (:`Started`
    (if (and (`self.IsHitCpp`) (`self.IsPlayerDieCpp`))
      _
      (elif (`self.CharDevelopMode`)
        (`self.ChangeSlotSkeletalServer` "RPistol2")
        (else
          (`self.OnQuickSlotSelected` 3))))))

(event `EnhancedInput|/Game/Level/TestLevel/CharTest/Player/Input/Action/IA_number7Weapon`
  (params (ActionValue :type Boolean) (ElapsedSeconds :type "Float (double-precision)") (TriggeredSeconds :type "Float (double-precision)") (InputAction :type "InputAction Object Reference" :default "/Game/Level/TestLevel/CharTest/Player/Input/Action/IA_number7Weapon.IA_number7Weapon"))
  ;[1 1 1] 무기 변경
  (:`Started`
    (if (and (`self.IsHitCpp`) (`self.IsPlayerDieCpp`))
      _
      (elif (`self.CharDevelopMode`)
        (`self.ChangeSlotSkeletalServer` "RRifle")
        (else
          (`self.OnQuickSlotSelected` 6))))))

(event `EnhancedInput|/Game/Level/TestLevel/CharTest/Player/Input/Action/IA_MainMove`
  (params (ActionValue :type "Vector2D Structure") (ElapsedSeconds :type "Float (double-precision)") (TriggeredSeconds :type "Float (double-precision)") (InputAction :type "InputAction Object Reference" :default "/Game/Level/TestLevel/CharTest/Player/Input/Action/IA_MainMove.IA_MainMove"))
  ;[1 1 1] 메시 동기화
  (:`Started`
    (`/Engine/EditorBlueprintResources/StandardMacros.DoOnce` false
      (:`Completed`
        (`|ExecutionSequence`
          (:`then_0`
            (`self.MeshInit` (`self.characterResultMesh`))
            (`self.Server`))
          (:`then_1`
            (bind _asbp_stsinstance (cast `/Game/STS/BP_STSInstance` (`GameplayStatics.GetGameInstance`)))
            (bind _returnvalue (`C_STSInstance.GetPlayerName` _asbp_stsinstance))
            (`self.NamesInit` (`KismetTextLibrary.Conv_StringToText` _returnvalue))
            (`self.ServerName`)))))))

(event `EnhancedInput|/Game/Level/TestLevel/CharTest/Player/Input/Action/IA_number2Weapon`
  (params (ActionValue :type Boolean) (ElapsedSeconds :type "Float (double-precision)") (TriggeredSeconds :type "Float (double-precision)") (InputAction :type "InputAction Object Reference" :default "/Game/Level/TestLevel/CharTest/Player/Input/Action/IA_number2Weapon.IA_number2Weapon"))
  (:`Started`
    ;[1 1 1] 무기 변경
    (if (and (`self.IsHitCpp`) (`self.IsPlayerDieCpp`))
      _
      (elif (`self.CharDevelopMode`)
        (`self.ChangeSlotMeshServer` "RSword" "/Game/Level/TestLevel/CharTest/Sword/Sw.Sw")
        (else
          (`self.OnQuickSlotSelected` 1))))))

(event `EnhancedInput|/Game/Level/TestLevel/CharTest/Player/Input/Action/IA_number5Weapon`
  (params (ActionValue :type Boolean) (ElapsedSeconds :type "Float (double-precision)") (TriggeredSeconds :type "Float (double-precision)") (InputAction :type "InputAction Object Reference" :default "/Game/Level/TestLevel/CharTest/Player/Input/Action/IA_number5Weapon.IA_number5Weapon"))
  ;[1 1 1] 무기 변경
  (:`Started`
    (if (and (`self.IsHitCpp`) (`self.IsPlayerDieCpp`))
      _
      (elif (`self.CharDevelopMode`)
        (`self.ChangeSlotSkeletalServer` "RPistol")
        (else
          (`self.OnQuickSlotSelected` 4))))))

(event `EnhancedInput|/Game/Level/TestLevel/CharTest/Player/Input/Action/IA_number8Weapon`
  (params (ActionValue :type Boolean) (ElapsedSeconds :type "Float (double-precision)") (TriggeredSeconds :type "Float (double-precision)") (InputAction :type "InputAction Object Reference" :default "/Game/Level/TestLevel/CharTest/Player/Input/Action/IA_number8Weapon.IA_number8Weapon"))
  ;[1 1 1] 무기 변경
  (:`Started`
    (if (and (`self.IsHitCpp`) (`self.IsPlayerDieCpp`))
      _
      (elif (`self.CharDevelopMode`)
        (`self.ChangeSlotSkeletalServer` "RShotgun")
        (else
          (`self.OnQuickSlotSelected` 7))))))

(event `self.ReceiveBeginPlay`
  (`|ExecutionSequence`
    (:`then_0`
      ;[1 1 1] 메시 동기화
      (`self.MeshInit` (`self.characterResultMesh`))
      (`self.MultMesh`)
      (`self.Server`))
    (:`then_1`
      ;[1 1 1] 캐릭터 스폰
      (bind _asbp_stsinstance (cast `/Game/STS/BP_STSInstance` (`GameplayStatics.GetGameInstance`)))
      (`self.K2_SetActorLocation` (`|GetArrayItem` (`C_STSInstance.GetPlayerSpawnLocation` _asbp_stsinstance) (`self.PlayerSpawnCheckToken`)) true true))
    (:`then_2`
      ;[1 1 1] 이름 텍스트 동기화
      (bind _asbp_stsinstance_2 (cast `/Game/STS/BP_STSInstance` (`GameplayStatics.GetGameInstance`)))
      (bind _returnvalue (`C_STSInstance.GetPlayerName` _asbp_stsinstance_2))
      (`self.NamesInit` (`KismetTextLibrary.Conv_StringToText` _returnvalue))
      (`self.MultName`)
      (`self.ServerName`))
    (:`then_3`
      ;[1 1 1] 미니맵 내에서 플레이어 컬러 변경
      (if (== (`self.GetController`) (`GameplayStatics.GetPlayerController` 0))
        (`PaperSpriteComponent.SetSpriteColor` (`self.MinimapIcon`) (struct :`G` 1.0 :`B` 0.019143 :`A` 1.0))
        (`|ExecutionSequence`
          (:`then_0`
            (bind _asbp_main_player_controller (cast `/Game/Level/TestLevel/CharTest/Player/MainController/BP_MainPlayerController` (`self.GetController`)))
            (`PlayerController.SetViewTargetWithBlend` _asbp_main_player_controller self 0.0 "VTBlend_Linear" 0.0 false))
          (:`then_1`
            (`self.SpawnMapCamera` (`KismetMathLibrary.MakeTransform` (`self.CameraLocation`)))
            (bind _returnvalue_2 (`|CreateWidget` "/Game/Level/TestLevel/UI/WidgetBP/InGame/WB_AttackBloodFX.WB_AttackBloodFX_C"))
            (`UserWidget.AddToViewport` _returnvalue_2 0)
            (set `self.NaviVec` (-53600.0 2430.0 0.0))))))))

(event `EnhancedInput|/Game/Level/TestLevel/CharTest/Player/Input/Action/IA_Zoom`
  (params (ActionValue :type Boolean) (ElapsedSeconds :type "Float (double-precision)") (TriggeredSeconds :type "Float (double-precision)") (InputAction :type "InputAction Object Reference" :default "/Game/Level/TestLevel/CharTest/Player/Input/Action/IA_Zoom.IA_Zoom"))
  (bind _curweapon (`self.CurWeapon`))
  ;[1 1 1] 에임 조준
  (:`Started`
    (`/Engine/EditorBlueprintResources/StandardMacros.IsValid` _curweapon
      (:`Is Valid`
        (if (not (`self.ISReload`))
          (bind _asbp_main_player_controller (cast `/Game/Level/TestLevel/CharTest/Player/MainController/BP_MainPlayerController` (`self.GetController`)))
          (`PlayerController.SetViewTargetWithBlend` _asbp_main_player_controller (`self.CurWeapon`) 0.0 "VTBlend_Linear" 0.0 false)
          (bind _asbp_ui_in_game_hud (cast `/Game/Level/TestLevel/UI/BP_UI_InGameHUD` (`PlayerController.GetHUD` _asbp_main_player_controller)))
          (`Widget.SetVisibility` (`/Game/Level/TestLevel/UI/WidgetBP/InGame/BP_HealthBar.CrossHair` (`/Game/Level/TestLevel/UI/BP_UI_InGameHUD.HPAndAimWidget` _asbp_ui_in_game_hud)) "Visible")))))
  (:`Canceled`
    (`/Engine/EditorBlueprintResources/StandardMacros.IsValid` _curweapon :!label _label
      (:`Is Valid`
        (bind _asbp_main_player_controller_2 (cast `/Game/Level/TestLevel/CharTest/Player/MainController/BP_MainPlayerController` (`self.GetController`)))
        (`PlayerController.SetViewTargetWithBlend` _asbp_main_player_controller_2 self 0.0 "VTBlend_Linear" 0.0 false)
        (bind _asbp_ui_in_game_hud_2 (cast `/Game/Level/TestLevel/UI/BP_UI_InGameHUD` (`PlayerController.GetHUD` _asbp_main_player_controller_2)))
        (`Widget.SetVisibility` (`/Game/Level/TestLevel/UI/WidgetBP/InGame/BP_HealthBar.CrossHair` (`/Game/Level/TestLevel/UI/BP_UI_InGameHUD.HPAndAimWidget` _asbp_ui_in_game_hud_2)) "Hidden"))))
  (:`Completed`
    (goto _label)))

(event `EnhancedInput|/Game/Level/TestLevel/CharTest/Player/Input/Action/IA_DebugN`
  (params (ActionValue :type Boolean) (ElapsedSeconds :type "Float (double-precision)") (TriggeredSeconds :type "Float (double-precision)") (InputAction :type "InputAction Object Reference" :default "/Game/Level/TestLevel/CharTest/Player/Input/Action/IA_DebugN.IA_DebugN")))

(event `test222`
  (`self.test1`))

(event `self.ReceiveTick`
  (params (DeltaSeconds :type "Float (single-precision)"))
  ;[1 1 1] 히트시 카메라 정리
  (if (or (`self.IsHitCpp`) (`self.IsPlayerDieCpp`))
    (bind _asbp_main_player_controller (cast `/Game/Level/TestLevel/CharTest/Player/MainController/BP_MainPlayerController` (`self.GetController`)))
    (`PlayerController.SetViewTargetWithBlend` _asbp_main_player_controller self 0.0 "VTBlend_Linear" 0.0 false)
    (bind _asbp_ui_in_game_hud (cast `/Game/Level/TestLevel/UI/BP_UI_InGameHUD` (`PlayerController.GetHUD` _asbp_main_player_controller)))
    (`Widget.SetVisibility` (`/Game/Level/TestLevel/UI/WidgetBP/InGame/BP_HealthBar.CrossHair` (`/Game/Level/TestLevel/UI/BP_UI_InGameHUD.HPAndAimWidget` _asbp_ui_in_game_hud)) "Hidden")))

(event `test1`
  (`self.K2_SetActorLocation` (`KismetMathLibrary.MakeVector` -58000.0 3500.0 -557.0)))

(fn `Get World Rotation`
  (returns (NewParam :type "Rotator Structure"))
  (return (`SceneComponent.K2_GetComponentRotation` (`self.CapsuleComponent`))))

(fn `GetForwardVector`
  (returns (NewParam :type "Vector Structure"))
  (return (`SceneComponent.GetForwardVector` (`self.CapsuleComponent`))))

(fn `GetWorldPostion`
  (returns (NewParam :type "Vector Structure"))
  (return (`SceneComponent.K2_GetComponentLocation` (`self.CapsuleComponent`))))

(fn `UserConstructionScript`)